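; AR actor that sets up a camera-feed shadow receiver material on its Cube mesh when play begins.
; A dynamic instance of BaseFeedScreen receives the AR camera frame as its texture, plus ARToolkit camera resolution and a portrait/landscape flag.
; BeginPlay then passes the Bike_d texture to ChangeColor as the initial color, though that function's body is empty.
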(event EventBeginPlay
  (Utilities|FlowControl|Sequence
    (:then_0
      ;[1 1 1] Set camera resolution for shadow receiver texture
      (bind _returnvalue (Class|ARToolkitComponent|GetCameraFrame))
      (bind _returnvalue_2 (Class|ARToolkitComponent|CreateDynamicMaterialInstance (Variables|Default|GetCube) "/Game/Materials/BaseFeedScreen.BaseFeedScreen"))
      (Class|ARToolkitComponent|SetTextureParameterValue _returnvalue_2 _returnvalue "Color")
      (bind (_webcamresx _webcamresy) (Class|ARToolkitComponent|GetCameraResolution (Variables|Default|GetARToolkit)))
      (Rendering|Material|SetScalarParameterValue _returnvalue_2 "CamResX" (Math|Conversions|ToFloat(Integer) _webcamresx) :!class /Script/Engine.MaterialInstanceDynamic)
      (Rendering|Material|SetScalarParameterValue _returnvalue_2 "CamResY" (Math|Conversions|ToFloat(Integer) _webcamresy) :!class /Script/Engine.MaterialInstanceDynamic)
      (switch Utilities|FlowControl|Switch|SwitchonEDeviceOrientation (Class|ARToolkitComponent|GetDeviceOrientation (Variables|Default|GetARToolkit))
        (:LANDSCAPE
          (Rendering|Material|SetScalarParameterValue _returnvalue_2 "IsPortrait" 0.0 :!class /Script/Engine.MaterialInstanceDynamic))
        (:PORTRAIT
          (Rendering|Material|SetScalarParameterValue _returnvalue_2 "IsPortrait" 1.0 :!class /Script/Engine.MaterialInstanceDynamic))))
    (:then_1
      ;[1 1 1] Set initial color
      (CallFunction|ChangeColor "/Game/HarleyDavidson/bike_d.bike_d"))))

(fn ConstructionScript)

(fn ChangeColor
  (params (Texture :type Texture%202D%20Object%20Reference)))