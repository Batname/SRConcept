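; Level surface actor for AR that feeds the device camera image into its surface material, apparently to act as a shadow receiver.
; On BeginPlay it creates a dynamic BaseFeedScreen material on SurfaceComponent and binds the camera frame as its Color texture.
; ChangeColor instead applies a Bike-based dynamic material with a given texture.
; The initial ChangeColor call and the camera resolution and orientation parameter setup are disconnected and never run.
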(event EventBeginPlay
  (Utilities|FlowControl|Sequence
    (:then_0
      ;[1 1 1] Set camera resolution for shadow receiver texture
      (bind _returnvalue (Class|ARToolkitComponent|GetCameraFrame))
      (bind _returnvalue_2 (Class|ARToolkitComponent|CreateDynamicMaterialInstance (Variables|Default|GetSurfaceComponent) "/Game/Materials/BaseFeedScreen.BaseFeedScreen"))
      (Class|ARToolkitComponent|SetTextureParameterValue _returnvalue_2 _returnvalue "Color"))))

(fn ConstructionScript)

(fn ChangeColor
  (params (NewParam :type Texture%202D%20Object%20Reference))
  (bind _returnvalue (Rendering|Material|CreateDynamicMaterialInstance (Variables|Default|GetSurfaceComponent) 0 "/Game/HarleyDavidson/bike.bike" :!class /Script/Engine.PrimitiveComponent))
  (Rendering|Material|SetTextureParameterValue _returnvalue "Texture" NewParam))